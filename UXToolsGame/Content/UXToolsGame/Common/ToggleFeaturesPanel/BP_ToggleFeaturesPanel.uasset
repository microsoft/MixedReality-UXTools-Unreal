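; BP_ToggleFeaturesPanel is a panel actor with a stats toggle button and a home button, both child actors bound on BeginPlay.
; The stats button runs the "stat unit" console command to toggle the performance display, and the home button opens the Loader level after a short delay.
; On EndPlay, a checked stats toggle reruns the command so the display does not stay on.
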(event Custom|Toggle%20Stats
  (params (Button :type Uxt%20Pressable%20Button%20Component%20Object%20Reference) (Pointer :type Uxt%20Pointer%20Component%20Object%20Reference))
  (Development|ExecuteConsoleCommand "stat unit" 0))

(event Custom|Load%20Loader
  (params (Button :type Uxt%20Pressable%20Button%20Component%20Object%20Reference) (Pointer :type Uxt%20Pointer%20Component%20Object%20Reference))
  (Utilities|FlowControl|Delay 0.25)
  (Game|OpenLevel(byName) "Loader"))

(event EventBeginPlay
  (bind _asbp_base_button (Utilities|Casting|CastToBP_BaseButton (Variables|/Script/Engine.ChildActorComponent|GetChildActor (Variables|Default|GetStatsButton))))
  (EventDispatchers|BindEventtoOnButtonPressed _asbp_base_button (delegate Custom|Toggle%20Stats))
  (bind _asbp_base_button_2 (Utilities|Casting|CastToBP_BaseButton (Variables|/Script/Engine.ChildActorComponent|GetChildActor (Variables|Default|GetHomeButton))))
  (EventDispatchers|BindEventtoOnButtonPressed _asbp_base_button_2 (delegate Custom|Load%20Loader)))

(event EventEndPlay
  (params (EndPlayReason :type EEndPlayReason%20Enum :default "Destroyed"))
  (bind _asbp_button_holo_lens_2toggle (Utilities|Casting|CastToBP_ButtonHoloLens2Toggle (Variables|/Script/Engine.ChildActorComponent|GetChildActor (Variables|Default|GetStatsButton))))
  (if (Variables|/Script/UXTools.UxtToggleStateComponent|GetbIsChecked (Variables|/UXTools/Buttons/HoloLens2/BP_ButtonHoloLens2Toggle.BP_ButtonHoloLens2Toggle_C|GetUxtToggleState _asbp_button_holo_lens_2toggle))
    (Development|ExecuteConsoleCommand "stat unit" 0)))

(fn ConstructionScript)