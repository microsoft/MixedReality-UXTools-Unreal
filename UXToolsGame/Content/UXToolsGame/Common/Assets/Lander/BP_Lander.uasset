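; BP_Lander is a lander actor whose landing gear folds and unfolds in response to a UXTools pinch slider.
; On BeginPlay it finds the UxtPinchSliderComponent on the referenced Slider, binds to its value updates and applies the current value.
; Each update linearly maps the inverted slider value to relative roll rotations on three arm and three leg components, which swing in opposite directions.
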(event Custom|UpdateLanderLegs
  (params (Slider :type Uxt%20Pinch%20Slider%20Component%20Object%20Reference) (NewValue :type Float%20%28single-precision%29))
  (Variables|Default|SetSliderValue NewValue)
  (CallFunction|UpdateLandingGear))

(event Custom|UpdateLandingGear
  (bind _slidervalue (Variables|Default|GetSliderValue))
  (bind _returnvalue (- 1.0 _slidervalue))
  (Utilities|FlowControl|Sequence
    (:then_0
      (Transformation|SetRelativeRotation (Variables|Default|GetLander_Arm) (Math|Rotator|MakeRotator (* (* _returnvalue 4e+01) -1.0) 0.0 0.0) false false))
    (:then_1
      (Transformation|SetRelativeRotation (Variables|Default|GetLander_Leg) (Math|Rotator|MakeRotator (* _returnvalue 9e+01) 0.0 0.0) false false))))

(event EventBeginPlay
  (bind _slider (Variables|Default|GetSlider))
  (bind _returnvalue (Actor|GetComponentbyClass _slider "/Script/UXTools.UxtPinchSliderComponent"))
  (Utilities|IsValid _returnvalue
    (:Is%20Valid
      (Variables|Default|SetSliderCompRef _returnvalue)
      (EventDispatchers|BindEventtoOnUpdateValue (Variables|Default|GetSliderCompRef) (delegate Custom|UpdateLanderLegs))
      (Variables|Default|SetSliderValue (Class|UxtPinchSliderComponent|GetSliderValue _returnvalue))
      (CallFunction|UpdateLandingGear))))

(fn ConstructionScript)