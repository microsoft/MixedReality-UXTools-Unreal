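; BP_Platonic is a UX Tools sample actor: a platonic solid mesh whose color is driven by three pinch sliders.
; The construction script creates a dynamic instance of a simple lit color material on the mesh.
; BeginPlay seeds Base Color from the red, green and blue slider values, then binds each slider's value-updated event.
; Each handler rewrites only its own channel, preserving the others.
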(event Custom|UpdateBlue
  (params (Slider :type Uxt%20Pinch%20Slider%20Component%20Object%20Reference) (NewValue :type Float%20%28single-precision%29))
  (bind _platonicdynamicmaterial (Variables|Default|GetPlatonicDynamicMaterial))
  ;[1 1 1] Updat Platonic Color on Slider interaction
  (bind _returnvalue (Rendering|Material|GetVectorParameterValue _platonicdynamicmaterial "Base Color" :!class /Script/Engine.MaterialInstanceDynamic))
  (Rendering|Material|SetVectorParameterValue _platonicdynamicmaterial "Base Color" (Utilities|Struct|MakeLinearColor (.r _returnvalue) (.g _returnvalue) NewValue (.a _returnvalue)) :!class /Script/Engine.MaterialInstanceDynamic))

(event Custom|UpdateRed
  (params (Slider :type Uxt%20Pinch%20Slider%20Component%20Object%20Reference) (NewValue :type Float%20%28single-precision%29))
  (bind _platonicdynamicmaterial (Variables|Default|GetPlatonicDynamicMaterial))
  ;[1 1 1] Updat Platonic Color on Slider interaction
  (bind _returnvalue (Rendering|Material|GetVectorParameterValue _platonicdynamicmaterial "Base Color" :!class /Script/Engine.MaterialInstanceDynamic))
  (Rendering|Material|SetVectorParameterValue _platonicdynamicmaterial "Base Color" (Utilities|Struct|MakeLinearColor NewValue (.g _returnvalue) (.b _returnvalue) (.a _returnvalue)) :!class /Script/Engine.MaterialInstanceDynamic))

(event Custom|UpdateGreen
  (params (Slider :type Uxt%20Pinch%20Slider%20Component%20Object%20Reference) (NewValue :type Float%20%28single-precision%29))
  (bind _platonicdynamicmaterial (Variables|Default|GetPlatonicDynamicMaterial))
  ;[1 1 1] Updat Platonic Color on Slider interaction
  (bind _returnvalue (Rendering|Material|GetVectorParameterValue _platonicdynamicmaterial "Base Color" :!class /Script/Engine.MaterialInstanceDynamic))
  (Rendering|Material|SetVectorParameterValue _platonicdynamicmaterial "Base Color" (Utilities|Struct|MakeLinearColor (.r _returnvalue) NewValue (.b _returnvalue) (.a _returnvalue)) :!class /Script/Engine.MaterialInstanceDynamic))

(event EventBeginPlay
  (bind _slider_blue (Variables|Default|GetSlider_Blue))
  (bind _slider_green (Variables|Default|GetSlider_Green))
  (bind _slider_red (Variables|Default|GetSlider_Red))
  (bind _returnvalue (Actor|GetComponentbyClass _slider_blue "/Script/UXTools.UxtPinchSliderComponent"))
  (bind _returnvalue_2 (Actor|GetComponentbyClass _slider_red "/Script/UXTools.UxtPinchSliderComponent"))
  (bind _returnvalue_3 (Actor|GetComponentbyClass _slider_green "/Script/UXTools.UxtPinchSliderComponent"))
  (Utilities|FlowControl|Sequence
    (:then_0
      ;[1 1 1] Get Current Slider Values as Update Platonic Color
      (Rendering|Material|SetVectorParameterValue (Variables|Default|GetPlatonicDynamicMaterial) "Base Color" (Utilities|Struct|MakeLinearColor (Class|UxtPinchSliderComponent|GetSliderValue (Actor|GetComponentbyClass (Variables|Default|GetSlider_Red) "/Script/UXTools.UxtPinchSliderComponent")) (Class|UxtPinchSliderComponent|GetSliderValue (Actor|GetComponentbyClass (Variables|Default|GetSlider_Green) "/Script/UXTools.UxtPinchSliderComponent")) (Class|UxtPinchSliderComponent|GetSliderValue (Actor|GetComponentbyClass (Variables|Default|GetSlider_Blue) "/Script/UXTools.UxtPinchSliderComponent")) 0.0) :!class /Script/Engine.MaterialInstanceDynamic))
    (:then_1
      ;[1 1 1] Bind Event to Slide On Value Changed
      (Utilities|IsValid _returnvalue_2
        (:Is%20Valid
          (EventDispatchers|BindEventtoOnValueUpdated _returnvalue_2 (delegate Custom|UpdateRed)))))
    (:then_2
      (Utilities|IsValid _returnvalue_3
        (:Is%20Valid
          (EventDispatchers|BindEventtoOnValueUpdated _returnvalue_3 (delegate Custom|UpdateGreen)))))
    (:then_3
      (Utilities|IsValid _returnvalue
        (:Is%20Valid
          (EventDispatchers|BindEventtoOnValueUpdated _returnvalue (delegate Custom|UpdateBlue)))))))

(fn ConstructionScript
  ;[1 1 1] Creat Dynamic Material for Platonic Mesh
  (bind _returnvalue (Rendering|Material|CreateDynamicMaterialInstance (Variables|Default|GetSM_Platonic) 0 "/UXTools/Materials/M_SimpleLit_Color.M_SimpleLit_Color" "None" :!class /Script/Engine.PrimitiveComponent))
  (Variables|Default|SetPlatonicDynamicMaterial _returnvalue))