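; Tooltip test actor that, judging by its name, serves as a stationary tracked target; all its events are empty, so it does not move itself.
; An unused MoveInCircle function holds logic to place it on a horizontal circle around a fixed offset from the world origin.
; That function derives the angle from a slowed, time-based pulsating value, then applies the position through both SetActorLocation and Teleport.
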(event EventBeginPlay)

(event Collision|EventActorBeginOverlap
  (params (OtherActor :type Actor%20Object%20Reference)))

(event EventTick
  (params (DeltaSeconds :type Float%20%28single-precision%29)))

(event EventEditorTick
  (params (DeltaTime :type Float%20%28single-precision%29)))

(fn ConstructionScript)

(fn MoveinCircle
  (bind _returnvalue (Utilities|Time|GetGameTimeinSeconds))
  (bind _returnvalue_2 (/ _returnvalue 1e+01))
  (bind _returnvalue_3 (Class|KismetMathLibrary|MakePulsatingValue _returnvalue_2 1.0 0.0))
  (bind _returnvalue_4 (Math|Float|MultiplybyPi _returnvalue_3))
  (bind _returnvalue_5 (* _returnvalue_4 2.0))
  (bind _returnvalue_6 (Math|Trig|Sin(Radians) _returnvalue_5))
  (bind _returnvalue_7 (Math|Trig|Cos(Radians) _returnvalue_5))
  (bind _returnvalue_8 (Math|Vector|MakeVector _returnvalue_6 _returnvalue_7 0.0))
  (bind _returnvalue_9 (* _returnvalue_8 1e+02))
  (bind _returnvalue_10 (+ (.y _returnvalue_9) 2e+02))
  (bind _returnvalue_11 (Math|Vector|MakeVector (.x _returnvalue_9) _returnvalue_10 (.z _returnvalue_9)))
  (Transformation|SetActorLocation _returnvalue_11 false false)
  (Transformation|Teleport _returnvalue_11 "0, 0, 0"))